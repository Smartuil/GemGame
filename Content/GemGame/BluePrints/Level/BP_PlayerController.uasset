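; Player controller for a gem-matching game that spawns the BP_Eater character and main UI, and resets play state on game start.
; Input slides the eater across seven lanes with a timeline.
; Upward line traces find gems to eat into a seven-slot stack shown in the game UI.
; Drawing respawns the last eaten gem at the column's end, then BP_GameMode clears matches; an animated fly variant is left unwired.
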(event `self.ReceiveBeginPlay`
  (bind _returnvalue (`|SpawnActorFromClass` "/Game/GemGame/BluePrints/Gem/BP_Eater.BP_Eater_C" (`KismetMathLibrary.MakeTransform` (-350.0 0.0 -500.0)) "Undefined" "OverrideRootScale" null null))
  (set `self.Ref_character` _returnvalue)
  (bind _asbp_game_mode (cast `/Game/GemGame/BluePrints/Level/BP_GameMode` (`GameplayStatics.GetGameMode`)))
  (set `self.RefGameMode` _asbp_game_mode)
  (bind _returnvalue_2 (`|CreateWidget` "/Game/GemGame/UI/UMG_MainUI.UMG_MainUI_C"))
  (bind _output_get (set `self.RefMainUI` _returnvalue_2))
  (`UserWidget.AddToViewport` _output_get 0))

(event `GemExplosion`)

(event `InputAction|characterMoveRight`
  (params (Key :type "Key Structure"))
  ;[1 1 1] CharacterMove
  (:`Pressed`
    (if (not (or (>= (`self.MoveCount`) 3) (`/Game/GemGame/BluePrints/Level/BP_GameMode.IsGameOver?` (`self.RefGameMode`))))
      (`self.MOveCharacter` true))))

(event `InputAction|characterMoveLeft`
  (params (Key :type "Key Structure"))
  ;[1 1 1] CharacterMove
  (:`Pressed`
    (if (not (or (`/Game/GemGame/BluePrints/Level/BP_GameMode.IsGameOver?` (`self.RefGameMode`)) (<= (`self.MoveCount`) -3)))
      (`self.MOveCharacter` false))))

(event `MoveCharacter`
  (params (`characterMoveRight?` :type Boolean))
  (bind _movecount (`self.MoveCount`))
  (bind _returnvalue (select `int` (+ (`self.MoveCount`) 3) :`0` 300.0 :`1` 200.0 :`2` 100.0 :`3` 0.0 :`4` -100.0 :`5` -200.0 :`6` -300.0 :!type "Float (single-precision)"))
  ;[1 1 1] CharacterMove
  (`/Engine/EditorBlueprintResources/StandardMacros.DoOnce` false :!label _label
    (:`Completed`
      (`self.ResetMoveInput`)
      (set `self.CharacterMoveRight?` `characterMoveRight?`)
      (bind (_direction _movevalue) (`Timeline|characterMoveTimeLine` :!via `PlayFromStart`)
        (:`Update`
          (`self.K2_SetActorLocation` (`self.Ref_character`) (`KismetMathLibrary.MakeVector` -350.0 (`KismetMathLibrary.Lerp` _returnvalue (+ _returnvalue (select `bool` (`self.CharacterMoveRight?`) :`false` 100.0 :`true` -100.0 :!type "Float (single-precision)")) _movevalue) -500.0) false false))
        (:`Finished`
          (if (`self.CharacterMoveRight?`)
            (`/Engine/EditorBlueprintResources/StandardMacros.IncrementInt` _movecount)
            (else
              (`/Engine/EditorBlueprintResources/StandardMacros.DecrementInt` _movecount))))))))

(event `ResetMoveInput`
  ;[1 1 1] CharacterMove
  (`KismetSystemLibrary.Delay` 0.1)
  (goto _label :!via `Reset`))

(event `EventCharacterEat`
  (bind _returnvalue (select `int` (+ (`self.MoveCount`) 3) :`0` 300.0 :`1` 200.0 :`2` 100.0 :`3` 0.0 :`4` -100.0 :`5` -200.0 :`6` -300.0 :!type "Float (single-precision)"))
  (if (not (or (>= (`self.GemEattenCount`) 7) (`/Game/GemGame/BluePrints/Level/BP_GameMode.IsGameOver?` (`self.RefGameMode`)))) :!label _label_2
    (bind (_outhit _returnvalue_2) (`KismetSystemLibrary.LineTraceSingleForObjects` :`Start` (`KismetMathLibrary.MakeVector` -350.0 _returnvalue -500.0) :`End` (`KismetMathLibrary.MakeVector` -350.0 _returnvalue 800.0) :`ObjectTypes` (`|MakeArray` "ObjectTypeQuery7" :!type "EObjectTypeQuery Enum") :`DrawDebugType` "ForDuration"))
    (if _returnvalue_2
      (bind _asbp_gem_master (cast `/Game/GemGame/BluePrints/Gem/BP_GemMaster` (`.HitActor` (`GameplayStatics.BreakHitResult` _outhit))))
      (for (_array_element _array_index) (`self.GemEattenArray`)
        (if (== _array_element 0)
          (bind _race (`/Game/GemGame/BluePrints/Gem/BP_GemMaster.race` _asbp_gem_master))
          (`KismetArrayLibrary.Array_Set` (`self.GemEattenArray`) _array_index _race)
          (`/Game/GemGame/UI/UMG_GameUI.EattingGemToSlot` (`self.RefGameUI`) _race _array_index)
          (`self.K2_DestroyActor` _asbp_gem_master)
          (`/Engine/EditorBlueprintResources/StandardMacros.IncrementInt` (`self.GemEattenCount`)
            (:`  `
              (break))))))))

(event `InputAction|characterEat`
  (params (Key :type "Key Structure"))
  (:`Pressed`
    (goto _label_2)))

(event `EventCharacterDraw`
  (bind _gemeattenarray (`self.GemEattenArray`))
  (bind _gemeattenarray_2 (`self.GemEattenArray`))
  (bind _returnvalue (- (`self.GemEattenCount`) 1))
  (bind _returnvalue_2 (- (`self.GemEattenCount`) 1))
  (bind _returnvalue_3 (select `int` (+ (`self.MoveCount`) 3) :`0` 300.0 :`1` 200.0 :`2` 100.0 :`3` 0.0 :`4` -100.0 :`5` -200.0 :`6` -300.0 :!type "Float (single-precision)"))
  (bind _returnvalue_4 (select `int` (`|GetArrayItem` (`self.GemEattenArray`) (- (`self.GemEattenCount`) 1)) :`0` "/Game/GemGame/BluePrints/Gem/BP_GemMaster.BP_GemMaster_C" :`1` "/Game/GemGame/BluePrints/Gem/BP_GemMaster.BP_GemMaster_C" :`2` "/Game/GemGame/BluePrints/Gem/BP_ChlidGem_02.BP_ChlidGem_02_C" :`3` "/Game/GemGame/BluePrints/Gem/BP_ChlidGem_03.BP_ChlidGem_03_C" :`4` "/Game/GemGame/BluePrints/Gem/BP_ChlidGem_04.BP_ChlidGem_04_C" :`5` "/Game/GemGame/BluePrints/Gem/BP_ChlidGem_05.BP_ChlidGem_05_C" :!type "Actor Class Reference"))
  (if (and (>= (`self.GemEattenCount`) 1) (not (`/Game/GemGame/BluePrints/Level/BP_GameMode.IsGameOver?` (`self.RefGameMode`)))) :!label _label_3
    (bind (_outhit _returnvalue_5) (`KismetSystemLibrary.LineTraceSingleForObjects` :`Start` (`KismetMathLibrary.MakeVector` -350.0 _returnvalue_3 -500.0) :`End` (`KismetMathLibrary.MakeVector` -350.0 _returnvalue_3 800.0) :`ObjectTypes` (`|MakeArray` "ObjectTypeQuery7" :!type "EObjectTypeQuery Enum") :`DrawDebugType` "ForDuration"))
    (if _returnvalue_5
      (bind _asbp_gem_master (cast `/Game/GemGame/BluePrints/Gem/BP_GemMaster` (`.HitActor` (`GameplayStatics.BreakHitResult` _outhit))))
      (bind (_returnvalue_x _returnvalue_y _returnvalue_z) (`KismetMathLibrary.BreakVector` (`self.K2_GetActorLocation` _asbp_gem_master)))
      (bind (_gemmoveendlocation_x _gemmoveendlocation_y _gemmoveendlocation_z) (`KismetMathLibrary.BreakVector` (`/Game/GemGame/BluePrints/Gem/BP_GemMaster.gemMoveEndLocation` _asbp_gem_master)))
      (bind _returnvalue_6 (`|SpawnActorFromClass` _returnvalue_4 (`KismetMathLibrary.MakeTransform` (`KismetMathLibrary.MakeVector` -350.0 _returnvalue_3 (select `bool` (`/Game/GemGame/BluePrints/Gem/BP_GemMaster.IsMoving?` _asbp_gem_master) :`false` (- _returnvalue_z 100.0) :`true` (- _gemmoveendlocation_z 100.0)))) "Undefined" "OverrideRootScale" null null))
      (set `self.DrawGemRaceRememer` (`|GetArrayItem` _gemeattenarray_2 _returnvalue_2))
      (`KismetArrayLibrary.Array_Set` _gemeattenarray_2 _returnvalue_2)
      (`/Game/GemGame/UI/UMG_GameUI.DrawGemFromSlot` (`self.RefGameUI`) _returnvalue_2)
      (`/Engine/EditorBlueprintResources/StandardMacros.DecrementInt` (`self.GemEattenCount`)
        (:`  `
          (`/Engine/EditorBlueprintResources/StandardMacros.IsValid` _returnvalue_6
            (:`Is Valid`
              (bind _asbp_gem_master_2 (cast `/Game/GemGame/BluePrints/Gem/BP_GemMaster` _returnvalue_6))
              (`/Game/GemGame/BluePrints/Gem/BP_GemMaster.FUC_GemHit` _asbp_gem_master_2 (`self.DrawGemRaceRememer`)))
            (:`Is Not Valid`
              _))
          (`/Game/GemGame/BluePrints/Level/BP_GameMode.CleanSameGem` (`self.RefGameMode`))))
      (else
        (bind _returnvalue_7 (`|SpawnActorFromClass` _returnvalue_4 (`KismetMathLibrary.MakeTransform` (`KismetMathLibrary.MakeVector` -350.0 _returnvalue_3 500.0)) "Undefined" "OverrideRootScale" null null))
        (set `self.DrawGemRaceRememer` (`|GetArrayItem` _gemeattenarray _returnvalue))
        (`KismetArrayLibrary.Array_Set` _gemeattenarray _returnvalue)
        (`/Game/GemGame/UI/UMG_GameUI.DrawGemFromSlot` (`self.RefGameUI`) _returnvalue)
        (`/Engine/EditorBlueprintResources/StandardMacros.DecrementInt` (`self.GemEattenCount`)
          (:`  `
            (`/Engine/EditorBlueprintResources/StandardMacros.IsValid` _returnvalue_7
              (:`Is Valid`
                (bind _asbp_gem_master_3 (cast `/Game/GemGame/BluePrints/Gem/BP_GemMaster` _returnvalue_7))
                (`/Game/GemGame/BluePrints/Gem/BP_GemMaster.FUC_GemHit` _asbp_gem_master_3 (`self.DrawGemRaceRememer`)))
              (:`Is Not Valid`
                _))
            (`/Game/GemGame/BluePrints/Level/BP_GameMode.CleanSameGem` (`self.RefGameMode`))))))))

(event `InputAction|characterDraw`
  (params (Key :type "Key Structure"))
  (:`Pressed`
    (goto _label_3)))

(event `ResetDrawGem`
  (bind _gemeattenarray (`self.GemEattenArray`))
  (bind _returnvalue (- (`self.GemEattenCount`) 1))
  (bind _returnvalue_2 (select `int` (+ (`self.MoveCount`) 3) :`0` 300.0 :`1` 200.0 :`2` 100.0 :`3` 0.0 :`4` -100.0 :`5` -200.0 :`6` -300.0 :!type "Float (single-precision)"))
  (bind _returnvalue_3 (select `int` (+ (`self.MoveCount`) 3) :`0` 300.0 :`1` 200.0 :`2` 100.0 :`3` 0.0 :`4` -100.0 :`5` -200.0 :`6` -300.0 :!type "Float (single-precision)"))
  (`KismetSystemLibrary.Delay` 0.2)
  (`/Game/GemGame/BluePrints/Level/BP_GameMode.CleanSameGem` (`self.RefGameMode`))
  (`/Engine/EditorBlueprintResources/StandardMacros.DoOnce` false :!via `Reset`
    (:`Completed`
      (`self.ResetDrawGem`)
      (bind (_outhit _returnvalue_4) (`KismetSystemLibrary.LineTraceSingleForObjects` :`Start` (`KismetMathLibrary.MakeVector` -350.0 _returnvalue_3 -500.0) :`End` (`KismetMathLibrary.MakeVector` -350.0 _returnvalue_3 800.0) :`ObjectTypes` (`|MakeArray` "ObjectTypeQuery7" :!type "EObjectTypeQuery Enum") :`DrawDebugType` "ForDuration"))
      (if _returnvalue_4
        (bind _asbp_gem_master (cast `/Game/GemGame/BluePrints/Gem/BP_GemMaster` (`.HitActor` (`GameplayStatics.BreakHitResult` _outhit)))
          (:`then`
            (if (`/Game/GemGame/BluePrints/Gem/BP_GemMaster.IsMoving?` _asbp_gem_master)
              (bind (_gemmoveendlocation_x _gemmoveendlocation_y _gemmoveendlocation_z) (`KismetMathLibrary.BreakVector` (`/Game/GemGame/BluePrints/Gem/BP_GemMaster.gemMoveEndLocation` _asbp_gem_master)))
              (set `self.DrawGemFlyLocation` (`KismetMathLibrary.MakeVector` -350.0 _gemmoveendlocation_y (- _gemmoveendlocation_z 100.0)))
              (else
                (bind (_returnvalue_x _returnvalue_y _returnvalue_z) (`KismetMathLibrary.BreakVector` (`self.K2_GetActorLocation` _asbp_gem_master)))
                (set `self.DrawGemFlyLocation` (`KismetMathLibrary.MakeVector` -350.0 _returnvalue_2 (- _returnvalue_z 100.0))))))
          (:`CastFailed`
            (set `self.DrawGemFlyLocation` (`KismetMathLibrary.MakeVector` -350.0 _returnvalue_2 500.0) :!label _label_4)))
        (else
          (goto _label_4)))
      (bind _returnvalue_5 (`|SpawnActorFromClass` (select `int` (`|GetArrayItem` (`self.GemEattenArray`) (- (`self.GemEattenCount`) 1)) :`0` "/Game/GemGame/BluePrints/Gem/BP_GemMaster.BP_GemMaster_C" :`1` "/Game/GemGame/BluePrints/Gem/BP_GemMaster.BP_GemMaster_C" :`2` "/Game/GemGame/BluePrints/Gem/BP_ChlidGem_02.BP_ChlidGem_02_C" :`3` "/Game/GemGame/BluePrints/Gem/BP_ChlidGem_03.BP_ChlidGem_03_C" :`4` "/Game/GemGame/BluePrints/Gem/BP_ChlidGem_04.BP_ChlidGem_04_C" :`5` "/Game/GemGame/BluePrints/Gem/BP_ChlidGem_05.BP_ChlidGem_05_C" :!type "Actor Class Reference") (`self.GetTransform` (`self.Ref_character`)) "Undefined" "OverrideRootScale" null null))
      (set `self.DrawGemRaceRememer` (`|GetArrayItem` _gemeattenarray _returnvalue))
      (`KismetArrayLibrary.Array_Set` _gemeattenarray _returnvalue)
      (`/Game/GemGame/UI/UMG_GameUI.DrawGemFromSlot` (`self.RefGameUI`) _returnvalue)
      (`/Engine/EditorBlueprintResources/StandardMacros.DecrementInt` (`self.GemEattenCount`)
        (:`  `
          (bind (_direction _flyvalue) (`Timeline|DrawGemFly` :!via `PlayFromStart`)
            (:`Update`
              (`self.K2_SetActorLocation` _returnvalue_5 (`KismetMathLibrary.VLerp` (`KismetMathLibrary.MakeVector` -350.0 (select `int` (+ (`self.MoveCount`) 3) :`0` 300.0 :`1` 200.0 :`2` 100.0 :`3` 0.0 :`4` -100.0 :`5` -200.0 :`6` -300.0 :!type "Float (single-precision)") -500.0) (`self.DrawGemFlyLocation`) _flyvalue) false false))
            (:`Finished`
              (bind _asbp_gem_master_2 (cast `/Game/GemGame/BluePrints/Gem/BP_GemMaster` _returnvalue_5))
              (`/Game/GemGame/BluePrints/Gem/BP_GemMaster.FUC_GemHit` _asbp_gem_master_2 (`self.DrawGemRaceRememer`)))))))))

(fn `FUC_GameStart`
  (locals (SetGemEattenArray :type "Array of Integer"))
  (bind _refgameui (`self.RefGameUI`))
  (`/Engine/EditorBlueprintResources/StandardMacros.IsValid` _refgameui
    (:`Is Valid`
      (if (not (`Widget.IsInViewport` _refgameui))
        (`UserWidget.AddToViewport` (`self.RefGameUI`) 0 :!label _label)))
    (:`Is Not Valid`
      (bind _returnvalue (`|CreateWidget` "/Game/GemGame/UI/UMG_GameUI.UMG_GameUI_C"))
      (set `self.RefGameUI` _returnvalue)
      (goto _label)))
  (set `self.PlayerScore` 0)
  (set `self.MoveCount` 0)
  (set `self.GemEattenCount` 0)
  (set `self.GemEattenArray` (`local.SetGemEattenArray`))
  (`self.K2_SetActorLocation` (`self.Ref_character`) (-350.0 0.0 -500.0) false false))

(fn `UserConstructionScript`)