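; Game mode for a seven-column gem-matching game, handling spawning, clearing, scoring, game over and a saved high-score table.
; A difficulty-timed loop spawns random rows at the top, pushing gems downward until a bottom line trace detects game over.
; Clearing three or more collected gems awards difficulty-scaled score, then per-column line traces measure gaps and slide gems upward to close them.
; Game over shows the panel and inserts the score into the ranking.
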(event `self.ReceiveBeginPlay`
  (bind _asbp_player_controller (cast `/Game/GemGame/BluePrints/Level/BP_PlayerController` (`GameplayStatics.GetPlayerController` 0)))
  (set `self.RefPlayerContoller` _asbp_player_controller)
  (`self.FUC_LoadGame`))

(event `CleanSameGem`
  (bind _refplayercontoller (`self.RefPlayerContoller`))
  (`KismetSystemLibrary.Delay` 0.1)
  (set `self.IsGemClearing?` true)
  (if (>= (`KismetArrayLibrary.Array_Length` (`self.saveGemHitCollection`)) 3)
    (for _array_element (`self.saveGemHitCollection`)
      (set `/Game/GemGame/BluePrints/Level/BP_PlayerController.PlayerScore` (+ (* (`/Game/GemGame/BluePrints/Gem/BP_GemMaster.score` _array_element) (select `int` (`self.DifficultLevel`) :`0` 1 :`1` 2 :`2` 3)) (`/Game/GemGame/BluePrints/Level/BP_PlayerController.PlayerScore` _refplayercontoller)) _refplayercontoller)
      (`GameplayStatics.SpawnEmitterAtLocation` "/Game/GemGame/ParticleSystem/P_ClearGem.P_ClearGem" (`self.K2_GetActorLocation` _array_element))
      (`self.K2_DestroyActor` _array_element)))
  (`KismetArrayLibrary.Array_Clear` (`self.saveGemHitCollection`))
  (`self.GemFall`))

(event `GemFall`
  (for _index (range 7)
    (bind _returnvalue (select `int` _index :`0` 300.0 :`1` 200.0 :`2` 100.0 :`3` 0.0 :`4` -100.0 :`5` -200.0 :`6` -300.0 :!type "Float (single-precision)"))
    (bind _outhits (`KismetSystemLibrary.LineTraceMultiForObjects` (`KismetMathLibrary.MakeVector` -350.0 _returnvalue 800.0) (`KismetMathLibrary.MakeVector` -350.0 _returnvalue -500.0) (`|MakeArray` "ObjectTypeQuery7" :!type "EObjectTypeQuery Enum")))
    (for _array_element _outhits
      (bind _asbp_gem_master (cast `/Game/GemGame/BluePrints/Gem/BP_GemMaster` (`.HitActor` (`GameplayStatics.BreakHitResult` _array_element))))
      (`/Engine/EditorBlueprintResources/StandardMacros.IsValid` (`self.DrawGemRemember`)
        (:`Is Valid`
          (bind (___2 _distance) (`self.DistanceCaculateForGrid` (`self.DrawGemRemember`) _asbp_gem_master))
          (if ___2
            (set `self.DrawGemDistanceRemember` (+ _distance (`self.DrawGemDistanceRemember`))))
          (if (`/Game/GemGame/BluePrints/Gem/BP_GemMaster.IsMoving?` _asbp_gem_master) :!label _label
            (bind (_gemmoveendlocation_x _gemmoveendlocation_y _gemmoveendlocation_z) (`KismetMathLibrary.BreakVector` (`/Game/GemGame/BluePrints/Gem/BP_GemMaster.gemMoveEndLocation` _asbp_gem_master)))
            (set `/Game/GemGame/BluePrints/Gem/BP_GemMaster.gemMoveEndLocation` (`KismetMathLibrary.MakeVector` -350.0 _gemmoveendlocation_y (+ _gemmoveendlocation_z (* (`self.DrawGemDistanceRemember`) 100.0))) _asbp_gem_master)
            (else
              (`/Game/GemGame/BluePrints/Gem/BP_GemMaster.GemMove` _asbp_gem_master 0 (`self.DrawGemDistanceRemember`)))))
        (:`Is Not Valid`
          (bind (_returnvalue_x _returnvalue_y _returnvalue_z) (`KismetMathLibrary.BreakVector` (`self.K2_GetActorLocation` _asbp_gem_master)))
          (if (<= _returnvalue_z 450.0)
            (set `self.DrawGemDistanceRemember` (+ (`KismetMathLibrary.FFloor` (/ (+ (- 500.0 _returnvalue_z) 20.0) 100.0)) (`self.DrawGemDistanceRemember`)))
            (goto _label)
            (else
              _))))
      (set `self.DrawGemRemember` _asbp_gem_master))
    (set `self.DrawGemRemember` null)
    (set `self.DrawGemDistanceRemember` 0))
  (set `self.IsGemClearing?` false))

(event `GemBuildLoopSystem`
  (`KismetSystemLibrary.Delay` (select `int` (`self.DifficultLevel`) :`0` 10.0 :`1` 5.0 :`2` 3.0 :!type "Float (single-precision)") :!label _label_2)
  (if (not (`self.IsGameOver?`))
    (`self.FUN_GemBuild`)
    (`self.CheckGameOver`)
    (goto _label_2)))

(event `CheckGameOver`
  (bind _refplayercontoller (`self.RefPlayerContoller`))
  (`KismetSystemLibrary.Delay` 1.0)
  (bind _outhit (`KismetSystemLibrary.LineTraceSingleForObjects` (-350.0 300.0 -500.0) (-350.0 -300.0 -500.0) (`|MakeArray` "ObjectTypeQuery7" :!type "EObjectTypeQuery Enum")))
  (cast `/Game/GemGame/BluePrints/Gem/BP_GemMaster` (`.HitActor` (`GameplayStatics.BreakHitResult` _outhit)))
  (set `self.IsGameOver?` true)
  (`/Game/GemGame/UI/UMG_GameUI.ShowGameOverPanel` (`/Game/GemGame/BluePrints/Level/BP_PlayerController.RefGameUI` _refplayercontoller))
  (set `PlayerController.bShowMouseCursor` true _refplayercontoller)
  (`self.FUC_CheckPlayerScore`))

(event `CleanAllGemInGame`
  (set `self.IsGameOver?` true)
  (bind _outactors (`GameplayStatics.GetAllActorsOfClass` "/Game/GemGame/BluePrints/Gem/BP_GemMaster.BP_GemMaster_C"))
  (for _array_element _outactors
    (`self.K2_DestroyActor` _array_element)))

(fn `DistanceCaculateForGrid`
  (params (GemUpon :type "/Game/GemGame/BluePrints/Gem/BP_GemMaster Object Reference") (GemBelow :type "/Game/GemGame/BluePrints/Gem/BP_GemMaster Object Reference"))
  (returns (`>=2` :type Boolean) (Distance :type Integer))
  (bind _returnvalue (`KismetMathLibrary.FFloor` (/ (+ (`KismetMathLibrary.VSize` (- (`self.K2_GetActorLocation` GemUpon) (`self.K2_GetActorLocation` GemBelow))) 20.0) 100.0)))
  (return (>= _returnvalue 2) (- _returnvalue 1)))

(fn `FUC_CheckPlayerScore`
  (locals (PlayerScoreRangeRemember :type "Array of Integer") (`IsScoreOnRange?` :type Boolean))
  (bind _playerscore (`/Game/GemGame/BluePrints/Level/BP_PlayerController.PlayerScore` (`self.RefPlayerContoller`)))
  (set `local.PlayerScoreRangeRemember` (`self.PlayerScoreRange`))
  (for (_array_element _array_index) (`local.PlayerScoreRangeRemember`)
    (if (`local.IsScoreOnRange?`)
      (`KismetArrayLibrary.Array_Set` (`self.PlayerScoreRange`) _array_index (`|GetArrayItem` (`local.PlayerScoreRangeRemember`) (- _array_index 1)))
      (elif (>= _playerscore _array_element)
        (set `local.IsScoreOnRange?` true)
        (`KismetArrayLibrary.Array_Set` (`self.PlayerScoreRange`) _array_index _playerscore)))))

(fn `FUC_GameStart`
  (for _index (range 14)
    (bind _returnvalue (>= _index 7))
    (`|SpawnActorFromClass` (select `int` (`KismetMathLibrary.RandomInteger` 5) :`0` "/Game/GemGame/BluePrints/Gem/BP_GemMaster.BP_GemMaster_C" :`1` "/Game/GemGame/BluePrints/Gem/BP_ChlidGem_02.BP_ChlidGem_02_C" :`2` "/Game/GemGame/BluePrints/Gem/BP_ChlidGem_03.BP_ChlidGem_03_C" :`3` "/Game/GemGame/BluePrints/Gem/BP_ChlidGem_04.BP_ChlidGem_04_C" :`4` "/Game/GemGame/BluePrints/Gem/BP_ChlidGem_05.BP_ChlidGem_05_C" :!type "Actor Class Reference") (`KismetMathLibrary.MakeTransform` (`KismetMathLibrary.MakeVector` -350.0 (select `int` (select `bool` _returnvalue :`false` _index :`true` (- _index 7)) :`0` 300.0 :`1` 200.0 :`2` 100.0 :`3` 0.0 :`4` -100.0 :`5` -200.0 :`6` -300.0 :!type "Float (single-precision)") (select `bool` _returnvalue :`false` 500.0 :`true` 400.0 :!type "Float (single-precision)"))) "Undefined" "OverrideRootScale" null null))
  (set `self.IsGameOver?` false)
  (`self.GemBuildLoopSystem`)
  (`/Game/GemGame/BluePrints/Level/BP_PlayerController.FUC_GameStart` (`self.RefPlayerContoller`)))

(fn `FUC_LoadGame`
  (bind _returnvalue (`GameplayStatics.DoesSaveGameExist` "SaveGame"))
  (if _returnvalue
    (bind _returnvalue_2 (`GameplayStatics.LoadGameFromSlot` "SaveGame"))
    (bind _asbp_save_game (cast `/Game/GemGame/BluePrints/Level/BP_SaveGame` _returnvalue_2))
    (bind _output_get (set `self.RefSaveGame` _asbp_save_game))
    (set `self.PlayerScoreRange` (`/Game/GemGame/BluePrints/Level/BP_SaveGame.SaveGamePlayerScoreRange` _output_get))
    (else
      (bind _returnvalue_3 (`GameplayStatics.CreateSaveGameObject` "/Game/GemGame/BluePrints/Level/BP_SaveGame.BP_SaveGame_C"))
      (set `self.RefSaveGame` _returnvalue_3))))

(fn `FUC_SaveGame`
  (set `/Game/GemGame/BluePrints/Level/BP_SaveGame.SaveGamePlayerScoreRange` (`self.PlayerScoreRange`) (`self.RefSaveGame`))
  (`GameplayStatics.SaveGameToSlot` (`self.RefSaveGame`) "SaveGame"))

(fn `FUN_GemBuild`
  (for _index (range 7)
    (`|SpawnActorFromClass` (select `int` (`KismetMathLibrary.RandomInteger` 5) :`0` "/Game/GemGame/BluePrints/Gem/BP_GemMaster.BP_GemMaster_C" :`1` "/Game/GemGame/BluePrints/Gem/BP_ChlidGem_02.BP_ChlidGem_02_C" :`2` "/Game/GemGame/BluePrints/Gem/BP_ChlidGem_03.BP_ChlidGem_03_C" :`3` "/Game/GemGame/BluePrints/Gem/BP_ChlidGem_04.BP_ChlidGem_04_C" :`4` "/Game/GemGame/BluePrints/Gem/BP_ChlidGem_05.BP_ChlidGem_05_C" :!type "Actor Class Reference") (`KismetMathLibrary.MakeTransform` (`KismetMathLibrary.MakeVector` -350.0 (select `int` _index :`0` 300.0 :`1` 200.0 :`2` 100.0 :`3` 0.0 :`4` -100.0 :`5` -200.0 :`6` -300.0 :!type "Float (single-precision)") 600.0)) "Undefined" "OverrideRootScale" null null))
  (bind _outactors (`GameplayStatics.GetAllActorsOfClass` "/Game/GemGame/BluePrints/Gem/BP_GemMaster.BP_GemMaster_C"))
  (for _array_element _outactors
    (if (`/Game/GemGame/BluePrints/Gem/BP_GemMaster.IsMoving?` _array_element)
      (bind (_gemmoveendlocation_x _gemmoveendlocation_y _gemmoveendlocation_z) (`KismetMathLibrary.BreakVector` (`/Game/GemGame/BluePrints/Gem/BP_GemMaster.gemMoveEndLocation` _array_element)))
      (set `/Game/GemGame/BluePrints/Gem/BP_GemMaster.gemMoveEndLocation` (`KismetMathLibrary.MakeVector` -350.0 _gemmoveendlocation_y (- _gemmoveendlocation_z 100.0)) _array_element)
      (else
        (`/Game/GemGame/BluePrints/Gem/BP_GemMaster.GemMove` _array_element 3 1))))
  (return))

(fn `UserConstructionScript`)