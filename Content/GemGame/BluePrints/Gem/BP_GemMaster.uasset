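; BP_GemMaster is the gem actor for a grid-based matching game, caching the player controller and game mode on BeginPlay.
; GemMove slides the gem along its up or right axis by a direction and distance, using a timeline lerp and an IsMoving flag.
; FUCGemHit recursively flood-fills same-Race neighbours via debug-drawn box traces at four arrow components, adding each unvisited match to the game mode's SaveGemHitCollection.
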(event `self.ReceiveBeginPlay`
  (bind _asbp_player_controller (cast `/Game/GemGame/BluePrints/Level/BP_PlayerController` (`GameplayStatics.GetPlayerController` 0)))
  (set `self.RefPlayerController` _asbp_player_controller)
  (bind _asbp_game_mode (cast `/Game/GemGame/BluePrints/Level/BP_GameMode` (`GameplayStatics.GetGameMode`)))
  (set `self.Ref_GameMode` _asbp_game_mode))

(event `GemMove`
  (params (MoveDirection :type Integer) (MoveDistance :type Integer))
  (bind _returnvalue (`self.K2_GetActorLocation`))
  (bind _returnvalue_2 (* MoveDistance 100.0))
  (bind _returnvalue_3 (* (`self.GetActorRightVector`) _returnvalue_2))
  (bind _returnvalue_4 (* (`self.GetActorUpVector`) _returnvalue_2))
  (set `self.IsMoving?` true)
  (set `self.gemMoveStartLocation` _returnvalue)
  (set `self.gemMoveEndLocation` (+ _returnvalue (select `int` MoveDirection :`0` (* _returnvalue_4 1.0) :`1` (* _returnvalue_3 1.0) :`2` (* _returnvalue_3 -1.0) :`3` (* _returnvalue_4 -1.0))))
  (bind (_direction _move_value) (`Timeline|MoveTimeLine` :!via `PlayFromStart`)
    (:`Update`
      (`self.K2_SetActorLocation` (`KismetMathLibrary.VLerp` (`self.gemMoveStartLocation`) (`self.gemMoveEndLocation`) _move_value)))
    (:`Finished`
      (set `self.IsMoving?` false))))

(fn `FUC_GemHit`
  (params (Race :type Integer))
  (bind _savegemhitcollection (`/Game/GemGame/BluePrints/Level/BP_GameMode.saveGemHitCollection` (`self.Ref_GameMode`)))
  (for _index (range 4)
    (bind _returnvalue (`SceneComponent.K2_GetComponentLocation` (select `int` _index :`0` (`self.ArrowUp`) :`1` (`self.ArrowDown`) :`2` (`self.ArrowLeft`) :`3` (`self.ArrowRight`))))
    (bind (_outhit _returnvalue_2) (`KismetSystemLibrary.BoxTraceSingleForObjects` :`Start` _returnvalue :`End` _returnvalue :`HalfSize` (10.0 10.0 10.0) :`ObjectTypes` (`|MakeArray` "ObjectTypeQuery7" :!type "EObjectTypeQuery Enum") :`DrawDebugType` "ForDuration"))
    (if _returnvalue_2
      (bind _asbp_gem_master (cast `/Game/GemGame/BluePrints/Gem/BP_GemMaster` (`.HitActor` (`GameplayStatics.BreakHitResult` _outhit))))
      (if (== Race (`/Game/GemGame/BluePrints/Gem/BP_GemMaster.race` _asbp_gem_master))
        (if (not (`KismetArrayLibrary.Array_Contains` _savegemhitcollection _asbp_gem_master))
          (`KismetArrayLibrary.Array_Add` _savegemhitcollection _asbp_gem_master)
          (`self.FUC_GemHit` _asbp_gem_master Race))))))

(fn `UserConstructionScript`)